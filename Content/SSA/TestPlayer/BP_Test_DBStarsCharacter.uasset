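; Test player character for exercising enemy AI, damage and bush hiding, with Enhanced Input movement and look.
; Health, healing and damage delegate to BPCDamageSystem, which drives a camera-facing health bar and an OnDeath binding.
; BushTracer overlaps toggle mesh custom depth and BPHideBush child-actor collision.
; Left click sphere-traces a melee hit; debug keys toggle enemy attacking/passive state, report damage to AI perception and emit noise with effects.
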(event OnComponentBeginOverlap(BushTracer)
  (params (OverlappedComponent :type Primitive%20Component%20Object%20Reference) (OtherActor :type Actor%20Object%20Reference) (OtherComp :type Primitive%20Component%20Object%20Reference) (OtherBodyIndex :type Integer) (bFromSweep :type Boolean) (SweepResult :type Hit%20Result%20Structure%20%28by%20ref%29))
  (Development|PrintString "Bush In")
  (Rendering|SetRenderCustomDepth (Variables|Character|GetMesh) true)
  (Collision|SetActorEnableCollision (Variables|/Script/Engine.ChildActorComponent|GetChildActor (Variables|Default|GetBP_HideBush)) true))

(event OnComponentEndOverlap(BushTracer)
  (params (OverlappedComponent :type Primitive%20Component%20Object%20Reference) (OtherActor :type Actor%20Object%20Reference) (OtherComp :type Primitive%20Component%20Object%20Reference) (OtherBodyIndex :type Integer))
  (Development|PrintString "Bush Out")
  (Rendering|SetRenderCustomDepth (Variables|Character|GetMesh) false)
  (Collision|SetActorEnableCollision (Variables|/Script/Engine.ChildActorComponent|GetChildActor (Variables|Default|GetBP_HideBush)) false))

(event Custom|E_Depth
  (Development|PrintString "Depth")
  (bind _asbp_dbs_enemy_v (Utilities|Casting|CastToBP_DBS_Enemy_V (Game|Player|GetPlayerPawn 0)))
  (Actor|DestroyActor _asbp_dbs_enemy_v))

(event Custom|Death
  (bind _mesh (Variables|Character|GetMesh))
  (Physics|SetSimulatePhysics _mesh false)
  (Collision|SetCollisionEnabled _mesh "QueryAndPhysics")
  (Input|DisableInput (Game|GetPlayerController 0)))

(event Custom|Blocked
  (Development|PrintString "Blocked"))

(event Input|EnhancedActionEvents|EnhancedInputActionIA_Test_Move
  (params (ActionValue :type Vector%202D%20Structure) (ElapsedSeconds :type Float%20%28double-precision%29) (TriggeredSeconds :type Float%20%28double-precision%29) (InputAction :type Input%20Action%20Object%20Reference :default "/Game/SSA/TestPlayer/IA_Test_Move.IA_Test_Move"))
  (bind _returnvalue (Pawn|GetControlRotation :!class /Script/Engine.Pawn))
  (Pawn|Input|AddMovementInput (Math|Vector|GetRightVector (Math|Rotator|MakeRotator (.roll _returnvalue) 0.0 (.yaw _returnvalue))) (.x ActionValue) false)
  (Pawn|Input|AddMovementInput (Math|Vector|GetForwardVector (Math|Rotator|MakeRotator 0.0 0.0 (.yaw (Pawn|GetControlRotation :!class /Script/Engine.Pawn)))) (.y ActionValue) false))

(event Input|EnhancedActionEvents|EnhancedInputActionIA_Test_Look
  (params (ActionValue :type Vector%202D%20Structure) (ElapsedSeconds :type Float%20%28double-precision%29) (TriggeredSeconds :type Float%20%28double-precision%29) (InputAction :type Input%20Action%20Object%20Reference :default "/Game/SSA/TestPlayer/IA_Test_Look.IA_Test_Look"))
  (Pawn|Input|AddControllerYawInput (.x ActionValue))
  (Pawn|Input|AddControllerPitchInput (.y ActionValue)))

(event EventDestroyed)

(event EventTick
  (params (DeltaSeconds :type Float%20%28single-precision%29))
  (bind _test_healthbar (Variables|Default|GetTEST_HealthBar))
  (bind _aswbp_hpbar (Utilities|Casting|CastToWBP_HPBar (UserInterface|GetWidget (Variables|Default|GetTEST_HealthBar))))
  (Progress|SetPercent (Variables|/Game/SSA/UI/Main/WBP_HPBar.WBP_HPBar_C|GetHealthBar _aswbp_hpbar) (/ (Variables|/Game/SSA/Interface/BPC_DamageSystem.BPC_DamageSystem_C|GetHealth (Variables|Default|GetBPC_DamageSystem)) 1e+02))
  (Transformation|SetWorldRotation _test_healthbar (Math|Rotator|FindLookatRotation (Transformation|GetWorldLocation _test_healthbar) (Transformation|GetWorldLocation (Variables|/Script/Engine.PlayerCameraManager|GetTransformComponent (Game|GetPlayerCameraManager 0)))) false false))

(event EventBeginPlay
  (bind _asplayer_controller (Utilities|Casting|CastToPlayerController (Pawn|GetController)))
  (Utilities|IsValid (PlayerController|LocalPlayerSubsystems|GetEnhancedInputLocalPlayerSubsystem _asplayer_controller)
    (:Is%20Valid
      (Input|AddMappingContext (PlayerController|LocalPlayerSubsystems|GetEnhancedInputLocalPlayerSubsystem _asplayer_controller) "/Game/SSA/TestPlayer/IMC_Test_Player.IMC_Test_Player" 0 "(bIgnoreAllPressedKeysUntilRelease=True,bForceImmediately=False,bNotifyUserSettings=False)"))))

(event Input|KeyboardEvents|1
  (params (Key :type Key%20Structure :default "None"))
  (:Pressed
    (Development|PrintString "Hello")
    (bind _returnvalue (Actor|GetActorOfClass "/Game/SSA/Enemy/Villager/BP_DBS_Enemy_V.BP_DBS_Enemy_V_C"))
    (bind _asaic_enemy_base (Utilities|Casting|CastToAIC_Enemy_base (AI|GetAIController _returnvalue)))
    (Utilities|FlowControl|FlipFlop
      (:A
        (Default|SetStateasAttacking _asaic_enemy_base self))
      (:B
        (Default|SetStateasPassive _asaic_enemy_base)))))

(event Input|KeyboardEvents|F
  (params (Key :type Key%20Structure :default "None"))
  (bind _returnvalue (Transformation|GetActorLocation))
  (:Pressed
    (Class|Actor|MakeNoise 1.0 self _returnvalue 0.0 "None")
    (Effects|SpawnEmitteratLocation "/Game/StarterContent/Particles/P_Explosion.P_Explosion" _returnvalue)
    (Audio|PlaySoundatLocation "/Engine/VREditor/Sounds/UI/Camera_Shutter.Camera_Shutter" _returnvalue "0, 0, 0" 1.0 1.0 0.0 0 0 0 0)))

(event Input|KeyboardEvents|2
  (params (Key :type Key%20Structure :default "None"))
  (:Pressed
    (bind _returnvalue (Actor|GetActorOfClass "/Game/SSA/Enemy/Villager/BP_DBS_Enemy_V.BP_DBS_Enemy_V_C"))
    (Class|AISenseDamage|ReportDamageEvent _returnvalue self 1e+01 (Transformation|GetActorLocation) "0, 0, 0" "None")))

(event Input|MouseEvents|LeftMouseButton
  (params (Key :type Key%20Structure :default "None"))
  (bind _returnvalue (Transformation|GetActorLocation))
  (:Pressed
    (bind (_outhit _returnvalue_2) (Collision|SphereTraceForObjects _returnvalue (+ _returnvalue (* (Transformation|GetActorForwardVector) 1e+02)) 5e+01 (Utilities|Array|MakeArray "ObjectTypeQuery3") false 0 "ForDuration" true "(R=1.000000,G=0.000000,B=0.000000,A=1.000000)" "(R=0.000000,G=1.000000,B=0.000000,A=1.000000)" 1.0))
    (if _returnvalue_2
      (Class|BPIDamagable|TakeDamage(Message) (.HitActor (Collision|BreakHitResult _outhit)) (Utilities|Struct|MakeS_DamageInfo 4e+01 "NewEnumerator1" "NewEnumerator0" false)))))

(event Input|KeyboardEvents|7
  (params (Key :type Key%20Structure :default "None"))
  (:Pressed
    (Development|PrintString "Hello")
    (CallFunction|EDepth)))

(fn ConstructionScript
  (EventDispatchers|BindEventtoOnDeath (Variables|Default|GetBPC_DamageSystem) (EventDispatchers|CreateEvent :!event Custom|Death)))

(fn GetCurrentHealth
  (return (Variables|/Game/SSA/Interface/BPC_DamageSystem.BPC_DamageSystem_C|GetHealth (Variables|Default|GetBPC_DamageSystem))))

(fn GetMaxHealth
  (return (Variables|/Game/SSA/Interface/BPC_DamageSystem.BPC_DamageSystem_C|GetMaxHealth (Variables|Default|GetBPC_DamageSystem))))

(fn Heal
  (params (Amount :type Float%20%28double-precision%29))
  (bind _newhealth (Default|Heal (Variables|Default|GetBPC_DamageSystem) Amount))
  (return _newhealth))

(fn TakeDamage
  (params (DamageInfo :type S%20Damage%20Info%20Structure))
  (bind _wasdamaged (Default|TakeDamage (Variables|Default|GetBPC_DamageSystem) DamageInfo))
  (return _wasdamaged))