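; Test top-down player character with click-to-move, a cooldown-limited montage attack, two item slots and a cursor-aimed skill.
; BPCDamageSystem holds health, which Tick mirrors to the HP bar and checks to trigger respawn on death.
; While alive, it faces its move goal when moving and the cursor when idle.
; Holding the skill drags a range indicator; releasing launches BP_SkillAtk toward the cursor and resets HitStack.
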(event Custom|AddItem
  (params (Item :type Actor%20Object%20Reference) (Healling :type Float%20%28double-precision%29))
  ;[0.15 0.15 0.15 0.5] 아이템 획득시 변수 저장
  (CallFunction|GetItem Item))

(event Custom|AtkStackSet
  ;[0.15 0.15 0.15 0.5] 공격이 명중시 스택이 쌓임
  (CallFunction|SetHitStack (Variables|Default|GetHit_Stack)))

(event Custom|Follow
  (params (GoalLocation :type Vector))
  ;[0.15 0.15 0.15 0.5] 컨트롤러에서 이동 이벤트 호출받아서 이동
  (if (Variables|Default|GetAlive)
    (AI|Navigation|SimpleMovetoLocation (Variables|Controller|GetPlayer%20Cotroller) GoalLocation)
    (Variables|Move|SetGoalVector GoalLocation)))

(event Custom|Move%20To
  (params (GoalLocation :type Vector))
  ;[0.15 0.15 0.15 0.5] 컨트롤러에서 이동 이벤트 호출받아서 이동
  (if (Variables|Default|GetAlive)
    (AI|Navigation|SimpleMovetoLocation (Variables|Controller|GetPlayer%20Cotroller) GoalLocation)
    (Variables|Move|SetGoalVector GoalLocation)))

(event Custom|OnDamgeMine
  (params (Damage :type Float%20%28double-precision%29))
  ;[0.15 0.15 0.15 0.5] 지뢰 아이템 대미지 활성화
  (if (not (Variables|Default|GetNowSpawn))
    (Variables|Default|SetCurrentHP (- (Variables|Default|GetCurrentHP) Damage))))

(event Custom|SetHP
  (bind _bpc_damagesystem (Variables|Default|GetBPC_DamageSystem))
  ;[0.15 0.15 0.15 0.5] 리스폰 시 체력을 다시 풀로 채우는 이벤트
  (Variables|/Game/SSA/Interface/BPC_DamageSystem.BPC_DamageSystem_C|SetHealth _bpc_damagesystem (Variables|/Game/SSA/Interface/BPC_DamageSystem.BPC_DamageSystem_C|GetMaxHealth _bpc_damagesystem)))

(event Input|EnhancedActionEvents|EnhancedInputActionIA_PlayerAtk
  (params (ActionValue :type Boolean) (ElapsedSeconds :type Float%20%28double-precision%29) (TriggeredSeconds :type Float%20%28double-precision%29) (InputAction :type Input%20Action%20Object%20Reference :default "/Game/ODH/InputAction/IA_PlayerAtk.IA_PlayerAtk"))
  ;[0.15 0.15 0.15 0.5] 살아 있는 상태에서 공격을 한 다음  일정 쿨타임 후 다시 공격이 이루어지게 만듦
  (:Completed
    (if (Variables|Default|GetAlive)
      (if (not (Variables|Default|GetAtk_CoolTime))
        (Variables|Default|SetAtk_CoolTime true)
        (Animation|Montage|PlayMontage (Variables|Character|GetMesh) "/Game/ODH/BP/Player/AM_Player_Montagu.AM_Player_Montagu" 1.0 0.0 "None" false
          (:then
            (Game|SpawnActorfromClass "/Game/ODH/BP/Player/BP_PlayerAtk.BP_PlayerAtk_C" (Transformation|GetWorldTransform (Variables|Default|GetAtkDirection)) "AlwaysSpawn" "MultiplyWithRoot" 0 0)
            ;;[0.15 0.15 0.15 0.5] 공격 쿨타임
            (Utilities|FlowControl|Delay 2.0)
            (Variables|Default|SetAtk_CoolTime false)))))))

(event Input|EnhancedActionEvents|EnhancedInputActionIA_PlayerSkill
  (params (ActionValue :type Boolean) (ElapsedSeconds :type Float%20%28double-precision%29) (TriggeredSeconds :type Float%20%28double-precision%29) (InputAction :type Input%20Action%20Object%20Reference :default "/Game/ODH/InputAction/IA_PlayerSkill.IA_PlayerSkill"))
  (bind _player_cotroller (Variables|Controller|GetPlayer%20Cotroller))
  (bind _hitresult (Game|Player|GetHitResultUnderCursorbyChannel _player_cotroller "TraceTypeQuery1" true))
  (bind _location (Collision|BreakHitResult _hitresult))
  ;[0.15 0 0.002558 0.5] 플레이어 스킬 발동 부분
  (:Triggered
    ;;[0.15 0.15 0.15 0.5] 공격 범위 액터가 있으면 마우스 위치로 옮겨준다
    (Utilities|IsValid (stale _returnvalue)
      (:Is%20Valid
        (Transformation|SetActorLocation (stale _returnvalue) (.Location (Collision|BreakHitResult (.HitResult (Game|Player|GetHitResultUnderCursorbyChannel (Variables|Controller|GetPlayer%20Cotroller) "TraceTypeQuery1" true)))) false false))))
  (:Started
    (if (>= (Variables|Default|GetHit_Stack) 0)
      ;;[0.15 0.15 0.15 0.5] 버튼을 눌렀을 때 공격 범위 액터를 마우스 위치에 소환
      (bind _returnvalue (Game|SpawnActorfromClass "/Game/ODH/BP/Player/BP_SkillRange.BP_SkillRange_C" (Math|Conversions|ToTransform(Vector) _location) "Undefined" "MultiplyWithRoot" 0 0))))
  (:Canceled
    ;;[0.15 0.15 0.15 0.5] 짧게 눌림 공격 범위 액터 삭제
    (Actor|DestroyActor _returnvalue))
  (:Completed
    (if (not false)
      (if (>= (Variables|Default|GetHit_Stack) 0)
        ;;[0.15 0.15 0.15 0.5] 스킬 스택이 찬 상태에서 일정 시간 이후 버튼을 때면 공격 오브젝트를 자신의 위치에 소환,
        ;; 자신의 위치와 마우스 위치를 전달해 포물선으로 날아가게 만들어준다. 이후 공격 범위 액터는 안보이게 없앤다.
        (Variables|Default|SetHit_Stack 0)
        (bind _returnvalue_2 (Game|SpawnActorfromClass "/Game/ODH/BP/Player/BP_SkillAtk.BP_SkillAtk_C" (Transformation|GetActorTransform) "Undefined" "MultiplyWithRoot" 0 0))
        (Default|OnSkill _returnvalue_2 (Transformation|GetActorLocation) _location)
        (Actor|DestroyActor _returnvalue)))))

(event Input|EnhancedActionEvents|EnhancedInputActionIA_Test
  (params (ActionValue :type Boolean) (ElapsedSeconds :type Float%20%28double-precision%29) (TriggeredSeconds :type Float%20%28double-precision%29) (InputAction :type Input%20Action%20Object%20Reference :default "/Game/ODH/InputAction/IA_Test.IA_Test"))
  ;[0.15 0.15 0.15 0.5] T로 플레이어 사망 임시 테스트
  (Variables|/Game/SSA/Interface/BPC_DamageSystem.BPC_DamageSystem_C|SetHealth (Variables|Default|GetBPC_DamageSystem) 0.0))

(event Input|EnhancedActionEvents|EnhancedInputActionIA_PlayerItem1
  (params (ActionValue :type Boolean) (ElapsedSeconds :type Float%20%28double-precision%29) (TriggeredSeconds :type Float%20%28double-precision%29) (InputAction :type Input%20Action%20Object%20Reference :default "/Game/ODH/InputAction/IA_PlayerItem1.IA_PlayerItem1"))
  ;[0.15 0.15 0.15 0.5] 아이템 사용 부분 아이템 배열을 순서대로 체크해서 해당 배열에 해당 아이템이 있으면 그것을 사용하고 빈자리로 만든다.
  (:Completed
    (bind _notmatch (CallFunction|UseHPItem (Utilities|Array|Get(acopy) (Variables|Default|GetItemArray)) (Variables|Default|GetCurrentHP) (stale Custom|AddItem Healling)))
    (if (not _notmatch)
      (CallFunction|UseMineItem (Utilities|Array|Get(acopy) (Variables|Default|GetItemArray)) (Transformation|GetActorLocation) (Game|GetPlayerCharacter 0)))))

(event Input|EnhancedActionEvents|EnhancedInputActionIA_PlayerItem2
  (params (ActionValue :type Boolean) (ElapsedSeconds :type Float%20%28double-precision%29) (TriggeredSeconds :type Float%20%28double-precision%29) (InputAction :type Input%20Action%20Object%20Reference :default "/Game/ODH/InputAction/IA_PlayerItem2.IA_PlayerItem2"))
  ;[0.15 0.15 0.15 0.5] 아이템 사용 부분 아이템 배열을 순서대로 체크해서 해당 배열에 해당 아이템이 있으면 그것을 사용하고 빈자리로 만든다.
  (:Completed
    (bind _notmatch (CallFunction|UseHPItem (Utilities|Array|Get(acopy) (Variables|Default|GetItemArray) 1) (Variables|Default|GetCurrentHP) 0.0))
    (if (not _notmatch)
      (CallFunction|UseMineItem (Utilities|Array|Get(acopy) (Variables|Default|GetItemArray) 1) (Transformation|GetActorLocation) (Game|GetPlayerCharacter 0)))))

(event EventBeginPlay
  ;[0.15 0.15 0.15 0.5] Controller를 받아서 변수에 저장
  (bind _asbp_top_down_player_controller (Utilities|Casting|CastToBP_TopDownPlayerController (Pawn|GetController)))
  (Variables|Controller|SetPlayer%20Cotroller _asbp_top_down_player_controller)
  ;[0.15 0.15 0.15 0.5] 초기화
  (CallFunction|Setting 5e+01)
  (bind _returnvalue (Actor|GetActorOfClass "/Game/ODH/BP/BP_GameManager.BP_GameManager_C"))
  (Variables|GameManager|SetGameManager _returnvalue)
  ;[0.15 0.15 0.15 0.5] 플레이어 HP UI 시각화
  (bind _aswbp_hpbar (Utilities|Casting|CastToWBP_HPBar (UserInterface|GetUserWidgetObject (Variables|Default|GetHPBar))))
  ;[0.15 0.15 0.15 0.5] 현재 체력 / 최대체력으로 체력바 변화
  (Progress|SetPercent (Variables|/Game/SSA/UI/Main/WBP_HPBar.WBP_HPBar_C|GetHealthBar _aswbp_hpbar) (/ (Variables|/Game/SSA/Interface/BPC_DamageSystem.BPC_DamageSystem_C|GetHealth (Variables|Default|GetBPC_DamageSystem)) 5e+01))
  (Variables|HPUI|SetHealthBar (Variables|/Game/SSA/UI/Main/WBP_HPBar.WBP_HPBar_C|GetHealthBar _aswbp_hpbar))
  (bind _asbp_test_dbs_game (Utilities|Casting|CastToBP_Test_DBS_Game (Game|GetGameMode)))
  (Variables|Default|SetUITest _asbp_test_dbs_game))

(event Collision|EventActorBeginOverlap
  (params (OtherActor :type Actor%20Object%20Reference))
  ;[0.15 0.15 0.15 0.5] 에너미 공격을 맞고 체력 감소
)

(event EventTick
  (params (DeltaSeconds :type Float%20%28single-precision%29))
  (bind _bpc_damagesystem (Variables|Default|GetBPC_DamageSystem))
  (bind _health (Variables|/Game/SSA/Interface/BPC_DamageSystem.BPC_DamageSystem_C|GetHealth _bpc_damagesystem))
  ;[0.15 0.15 0.15 0.5] 체력 변화에 맞게 언제나 보여줌
  (Progress|SetPercent (Variables|HPUI|GetHealthBar) (/ _health 5e+01))
  ;[0.15 0.15 0.15 0.5] 살아있는 상태인지 확인
  (bind _alive (CallFunction|CheckAlive (Variables|Default|GetAlive) _health self))
  (if _alive
    ;[0.15 0.15 0.15 0.5] 리스폰 상태인지 체크하여 리스폰 상태일 경우 시간을 체크해서 일정 시간 이상이 되면 해제됨
    (CallFunction|CheckNowSpawn (Variables|Default|GetNowSpawn) (Variables|Default|GetRespawnCurrentTime))
    (if (> (Math|Vector|VectorLength (Transformation|GetVelocity)) 0.1)
      ;[0.15 0.15 0.15 0.5] 마지막으로 향하는 방향을 향해 시선을 고정한다
      (Transformation|SetActorRotation (Math|Rotator|MakeRotator 0.0 0.0 (.yaw (Math|Rotator|FindLookatRotation (Transformation|GetActorLocation) (Variables|Move|GetGoalVector)))))
      (else
        ;[0.15 0.15 0.15 0.5] 캐릭터가 마우스 포인터를 향해 바라봄
        (Transformation|SetActorRotation (Math|Rotator|MakeRotator 0.0 0.0 (.yaw (Math|Rotator|FindLookatRotation (Transformation|GetActorLocation) (.Location (Collision|BreakHitResult (.HitResult (Game|Player|GetHitResultUnderCursorbyChannel (Variables|Controller|GetPlayer%20Cotroller) "TraceTypeQuery1" true))))))))))
    (else
      ;[0.15 0.15 0.15 0.5] 죽으면 캐릭터 리스폰 및 데스 카운트 추가
      (Rendering|SetVisibility (Variables|Character|GetMesh) false false)
      (CallFunction|Respawn (Variables|Default|GetAlive) (Variables|Default|GetRespawnDelayTime) (Variables|Character|GetMesh) (Game|GetPlayerCharacter 0)))))

(fn ConstructionScript)

(fn CharaRotation
  (params (NowMoving :type Boolean))
  (if (not NowMoving)
    ;[0.15 0.15 0.15 0.5] 캐릭터가 마우스 포인터를 향해 바라봄
    (Transformation|SetActorRotation (Math|Rotator|MakeRotator 0.0 0.0 (.yaw (Math|Rotator|FindLookatRotation (Transformation|GetActorLocation) (.Location (Collision|BreakHitResult (.HitResult (Game|Player|GetHitResultUnderCursorbyChannel (Variables|Controller|GetPlayer%20Cotroller) "TraceTypeQuery1" true))))))))))

(fn OutPut
  (return false))

(fn GetCurrentHealth
  (return (Variables|Default|GetCurrentHP)))

(fn GetMaxHealth
  (return (Variables|Default|GetMAX_HP)))

(fn Heal
  (params (Amount :type Float%20%28double-precision%29))
  (bind _currenthp (CallFunction|UseHPItem 0 0.0 0.0))
  (return _currenthp))

(fn TakeDamage
  (params (DamageInfo :type S%20Damage%20Info%20Structure))
  (bind _wasdamaged (Default|TakeDamage (Variables|Default|GetBPC_DamageSystem) DamageInfo))
  (return _wasdamaged))