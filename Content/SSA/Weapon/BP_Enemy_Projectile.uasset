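; Enemy projectile actor that flies straight along its forward vector and ignores its owner for collision.
; Tick moves it manually by speed and delta time, without sweeping.
; A box collision hit broadcasts the impact event, spawns an emitter at the hit, plays a sound at world origin and destroys the actor.
; Damage is left to impact listeners; the sphere-trace damage nodes here are disconnected.
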(event OnComponentHit(BoxCollision)
  (params (HitComponent :type Primitive%20Component%20Object%20Reference) (OtherActor :type Actor%20Object%20Reference) (OtherComp :type Primitive%20Component%20Object%20Reference) (NormalImpulse :type Vector :default "0, 0, 0") (Hit :type Hit%20Result%20Structure%20%28by%20ref%29))
  (Default|CallOnProjectileimpact OtherActor Hit)
  ;[0.15 0.15 0.15 0.5] 이펙트 추가
  (Effects|SpawnEmitteratLocation (Variables|Effect|GetEmitter%20Template) (.Location (Collision|BreakHitResult Hit)))
  ;[0.15 0.15 0.15 0.5] 소리 작업
  (Audio|PlaySoundatLocation (Variables|Effect|GetSound) "0, 0, 0" "0, 0, 0" 1.0 1.0 0.0 0 0 0 0)
  (Actor|DestroyActor))

(event EventBeginPlay
  (Collision|IgnoreActorwhenMoving (Variables|Default|GetBox%20Collision) (Components|GetOwner) true))

(event EventTick
  (params (DeltaSeconds :type Float%20%28single-precision%29))
  (Transformation|SetActorLocation (+ (Transformation|GetActorLocation) (* (* (Transformation|GetActorForwardVector) (Variables|Default|GetSpeed)) (Utilities|Time|GetWorldDeltaSeconds))) false false))

(fn ConstructionScript)