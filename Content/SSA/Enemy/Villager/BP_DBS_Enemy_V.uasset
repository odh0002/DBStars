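; Villager enemy character whose health, healing and damage run through BPCDamageSystem, with a health bar widget overhead.
; Exposes patrol route, ideal range and movement speed, can wield a socketed sword, and chases the player with AIMoveTo.
; Attack plays a montage while a sphere trace immediately deals random damage and updates the player's damage widget; notify-triggered launches have zero velocity.
; Spawn and death update the game mode's alive count; death also requests a respawn.
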(event Custom|Attack
  (bind _returnvalue (Transformation|GetActorLocation))
  (bind _returnvalue_2 (Transformation|GetActorLocation))
  (bind _randomdamage (Variables|Default|GetRandomDamage))
  (bind _returnvalue_3 (Math|Random|RandomIntegerinRange 500 _randomdamage))
  (bind _returnvalue_4 (Math|Conversions|ToFloat(Integer) _returnvalue_3))
  (bind _s_damageinfo (Utilities|Struct|MakeS_DamageInfo _returnvalue_4 "NewEnumerator1" "NewEnumerator1" true))
  (Utilities|FlowControl|Sequence
    (:then_0
      (Animation|Montage|PlayMontage (Variables|Character|GetMesh) "/Game/SSA/Enemy/Enemy_Asset/Villager/Animation/A_Attack_Montage.A_Attack_Montage"
        (:OnCompleted
          (Default|CallOnAttackEnd :!label _label))
        (:OnInterrupted
          (goto _label))
        (:OnNotifyBegin
          (bind (_outhit _returnvalue_5) (Collision|SphereTraceByChannel _returnvalue (+ _returnvalue (* (Math|Vector|GetForwardVector (Transformation|GetActorRotation)) 5e+02)) 3e+01 "TraceTypeQuery3" false 0 "None" true "(R=1.000000,G=0.000000,B=0.000000,A=1.000000)" "(R=0.000000,G=1.000000,B=0.000000,A=1.000000)" 0.5))
          (if _returnvalue_5
            (bind _asbp_player (Utilities|Casting|CastToBP_Player (.HitActor (Collision|BreakHitResult _outhit))))
            (Character|LaunchCharacter _asbp_player "0, 0, 0" false false)))))
    (:then_1
      (bind (_outhit_2 _returnvalue_6) (Collision|SphereTraceForObjects _returnvalue_2 (+ _returnvalue_2 (* (Transformation|GetActorForwardVector) 1e+02)) 5e+01 (Utilities|Array|MakeArray "ObjectTypeQuery7") false 0 "ForOneFrame" true "(R=1.000000,G=0.000000,B=0.000000,A=1.000000)" "(R=0.000000,G=1.000000,B=0.000000,A=1.000000)" 1.0))
      (if _returnvalue_6
        (Class|BPIDamagable|TakeDamage(Message) (.HitActor (Collision|BreakHitResult _outhit_2)) _s_damageinfo)
        (bind _asbp_player_2 (Utilities|Casting|CastToBP_Player (Game|Player|GetPlayerPawn 0)))
        (bind _aswbp_damage (Utilities|Casting|CastToWBP_Damage (UserInterface|GetWidget (Variables|/Game/ODH/BP/Player/BP_Player.BP_Player_C|GetDamageWidget _asbp_player_2))))
        (Default|ApplyDamage _aswbp_damage (Utilities|Text|ToText(Float) (.Amount (Utilities|Struct|BreakS_DamageInfo _s_damageinfo)) "HalfToEven"))))))

(event Custom|WieldSword
  (bind _returnvalue (Game|SpawnActorfromClass "/Game/SSA/Weapon/BP_Sword.BP_Sword_C" (Transformation|GetActorTransform) "DontSpawnIfColliding" "MultiplyWithRoot" 0 0))
  (Transformation|AttachComponentToComponent _returnvalue (Variables|Character|GetMesh) "Hand_r_Sword_Socket" "SnapToTarget" "SnapToTarget" "SnapToTarget" true)
  (Variables|AI|SetIsWiedingSword true))

(event Custom|FollowPlayer
  (bind _returnvalue (Transformation|GetActorLocation))
  (AI|AIMoveTo self "0, 0, 0" (Game|GetPlayerCharacter 0) 3e+02 false
    (:OnSuccess
      (if (Variables|Default|GetcanAttack?)
        (Animation|Montage|PlayMontage (Variables|Character|GetMesh) "/Game/SSA/Enemy/Enemy_Asset/Villager/Animation/A_Attack_Montage.A_Attack_Montage"
          (:then
            (Variables|Default|SetcanAttack? false))
          (:OnCompleted
            (Variables|Default|SetcanAttack? true :!label _label))
          (:OnInterrupted
            (goto _label))
          (:OnNotifyBegin
            (bind (_outhit _returnvalue_2) (Collision|SphereTraceByChannel _returnvalue (+ _returnvalue (* (Math|Vector|GetForwardVector (Transformation|GetActorRotation)) 3e+02)) 3e+01 "TraceTypeQuery3" false 0 "None" true "(R=1.000000,G=0.000000,B=0.000000,A=1.000000)" "(R=0.000000,G=1.000000,B=0.000000,A=1.000000)" 0.5))
            (if _returnvalue_2
              (bind _asbp_player (Utilities|Casting|CastToBP_Player (.HitActor (Collision|BreakHitResult _outhit))))
              (Character|LaunchCharacter _asbp_player (+ (* (Math|Vector|GetForwardVector (Transformation|GetActorRotation)) "") (Math|Vector|MakeVector 0.0 0.0 0.0)) false false))))))))

(event Custom|OnDeath_Event
  (EventDispatchers|AssignOnDeath (Variables|Default|GetBPC_DamageSystem) (delegate Custom|OnDeath_Event)))

(event Custom|Death
  (Development|PrintString "DEAD")
  (Pawn|Components|CharacterMovement|DisableMovement (Variables|Character|GetCharacterMovement))
  (Utilities|FlowControl|Delay 2.0)
  (bind _asbp_dbs_game (Utilities|Casting|CastToBP_DBS_Game (Game|GetGameMode)))
  (Math|Integer|DecrementInt (Variables|/Game/SSA/BP_DBS_Game.BP_DBS_Game_C|GetEnemeisAlive _asbp_dbs_game)
    (:%20%20
      (Default|CastRespawnEnemy _asbp_dbs_game)
      (Actor|DestroyActor))))

(event Custom|Blocked
  (Development|PrintString "Blocked"))

(event Custom|DamageResponse
  (Development|PrintString "Hello"))

(event Custom|HpDown
  (params (Player :type Actor%20Object%20Reference)))

(event Custom|DamagePlayer
  (params (OtherActor :type Actor%20Object%20Reference) (Hit :type Hit%20Result%20Structure))
  (Class|BPIDamagable|TakeDamage(Message) OtherActor (Utilities|Struct|MakeS_DamageInfo 1e+01 "NewEnumerator1" "NewEnumerator2" false)))

(event EventDestroyed)

(event EventBeginPlay
  (Utilities|FlowControl|Sequence
    (:then_0
      (bind _returnvalue (UserInterface|CreateWidget "/Game/SSA/UI/Main/WBP_HPBar.WBP_HPBar_C" 0 self))
      (UserInterface|SetWidget (Variables|Default|GetHealthBar) _returnvalue))
    (:then_1
      (bind _asbp_dbs_game (Utilities|Casting|CastToBP_DBS_Game (Game|GetGameMode)))
      (Math|Integer|IncrementInt (Variables|/Game/SSA/BP_DBS_Game.BP_DBS_Game_C|GetEnemeisAlive _asbp_dbs_game)))))

(event EventTick
  (params (DeltaSeconds :type Float%20%28single-precision%29))
  (bind _aswbp_hpbar (Utilities|Casting|CastToWBP_HPBar (UserInterface|GetWidget (Variables|Default|GetHealthBar))))
  (bind _retrun_value (Default|GetPercent _aswbp_hpbar))
  (Progress|SetPercent (Variables|/Game/SSA/UI/Main/WBP_HPBar.WBP_HPBar_C|GetHealthBar _aswbp_hpbar) _retrun_value))

(event EventGetScore)

(fn ConstructionScript
  (EventDispatchers|BindEventtoOnDeath (Variables|Default|GetBPC_DamageSystem) (EventDispatchers|CreateEvent :!event Custom|Death)))

(fn GetCurrentHealth
  (return (Variables|/Game/SSA/Interface/BPC_DamageSystem.BPC_DamageSystem_C|GetHealth (Variables|Default|GetBPC_DamageSystem))))

(fn GetIdealRange
  (return 1.5e+02 6e+02))

(fn GetMaxHealth
  (return (Variables|/Game/SSA/Interface/BPC_DamageSystem.BPC_DamageSystem_C|GetMaxHealth (Variables|Default|GetBPC_DamageSystem))))

(fn GetPatrolRoute
  (return (Variables|AI|GetPatrolRoute)))

(fn Heal
  (params (Amount :type Float%20%28double-precision%29))
  (bind _newhealth (Default|Heal (Variables|Default|GetBPC_DamageSystem) Amount))
  (return _newhealth))

(fn SetMovementSpeed
  (params (Speed :type E_MovementSpeed%20Enum :default "NewEnumerator0"))
  (bind _output_get (Variables|/Script/Engine.CharacterMovementComponent|SetMaxWalkSpeed (Variables|Character|GetCharacterMovement) (Utilities|Select :Index Speed :NewEnumerator0 0.0 :NewEnumerator1 3.4e+02 :NewEnumerator2 3.4e+02 :NewEnumerator3 3.4e+02)))
  (return _output_get))

(fn TakeDamage
  (params (DamageInfo :type S%20Damage%20Info%20Structure))
  (bind _wasdamaged (Default|TakeDamage (Variables|Default|GetBPC_DamageSystem) DamageInfo))
  (return _wasdamaged))