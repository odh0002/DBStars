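; Enemy character that uses PawnSensing to spot a pawn, then runs AI MoveTo toward the player character.
; On arrival a CanAttack check gates the attack montage, but the flag is cleared before the move and set true only inside that check.
; While IsSeeingPlayer is set, Tick stops active movement every frame, working against the chase.
; A separate Attack event also plays the montage on the mesh.
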(event OnSeePawn(PawnSensing)
  (params (Pawn :type Pawn%20Object%20Reference))
  (Variables|Default|SetisSeeingPlayer? true)
  (CallFunction|FollowPlayer))

(event Custom|Attack
  (Animation|Montage|PlayMontage (Variables|Character|GetMesh) "/Game/SSA/Enemy_Asset/EnemyAnimamtion/Montage/Attack_Montage.Attack_Montage"))

(event Custom|FollowPlayer
  (Variables|Default|SetcanAttack? false)
  (if (Variables|Default|GetisSeeingPlayer?)
    (AI|AIMoveTo self "0, 0, 0" (Game|GetPlayerCharacter 0) 1.6e+02 false
      (:then
        (if (Variables|Default|GetcanAttack?)
          (Variables|Default|SetcanAttack? true)
          (bind _returnvalue (Animation|PlayAnimMontage "/Game/SSA/Enemy_Asset/EnemyAnimamtion/Montage/Attack_Montage.Attack_Montage" 1.0 "None"))
          (Utilities|FlowControl|Delay _returnvalue)
          (Variables|Default|SetcanAttack? false))))
    (else
      (Variables|Default|SetisSeeingPlayer? false))))

(event EventBeginPlay)

(event Collision|EventActorBeginOverlap
  (params (OtherActor :type Actor%20Object%20Reference)))

(event EventTick
  (params (DeltaSeconds :type Float%20%28single-precision%29))
  (if (Variables|Default|GetisSeeingPlayer?)
    (Class|NavMovementInterface|StopActiveMovement (Variables|Character|GetCharacterMovement))))

(fn ConstructionScript)