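; BP_PlayerRespawnPlace respawns a dead player near a given respawn actor.
; Its CharacterRespawn event calls Respawn, which, when Alive is false, finds BP_Player with GetActorOfClass and moves it to a random point in a small box around that actor.
; It then sets the player's Alive flag back to true.
; The node that adds health to CurrentHP is unconnected, so health is unchanged.
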(event Custom|Character%20Respawn
  (params (Alive :type Boolean) (RespawnActor :type Actor%20Object%20Reference))
  ;[0.15 0.15 0.15 0.5] 플레이어 리스폰 이벤트
  (CallFunction|Respawn Alive RespawnActor))

(event EventBeginPlay)

(event Collision|EventActorBeginOverlap
  (params (OtherActor :type Actor%20Object%20Reference)))

(event EventTick
  (params (DeltaSeconds :type Float%20%28single-precision%29)))

(fn ConstructionScript)

(fn Respawn
  (params (Alive :type Boolean) (RespawnActor :type Actor%20Object%20Reference))
  ;[0.15 0.15 0.15 0.5] 만약 죽어있는 상태면 클래스를 받아옴
  (if (not Alive)
    (bind _returnvalue (Actor|GetActorOfClass "/Game/ODH/BP/Player/BP_Player.BP_Player_C"))
    ;[0.15 0.15 0.15 0.5] 플레이어의 위치를 이동 시킨 다음 살아있음과 체력을 다시 리셋시켜줌
    (Transformation|SetActorRelativeLocation _returnvalue (Math|Random|RandomPointinBoundingBox (Transformation|GetActorLocation RespawnActor) (Math|Vector|MakeVector 2e+01 2e+01 0.0)))
    (Variables|/Game/ODH/BP/BP_CharacterStat.BP_CharacterStat_C|SetAlive _returnvalue true)))