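; Character stat actor holding alive state, capped hit stack, healing and a two-slot item inventory.
; CheckAlive reports death to BP_DBS_Game; Respawn uses a delta-time timer, then restores BP_Player at a random BP_PlayerRespawnPlace, resetting items and starting a spawn-state window timed by CheckNowSpawn.
; Item functions update inventory UI slots, consume HP items and spawn ground mines.
; Enemy respawn is only a cast stub, and Setting's HP initialization is disconnected.
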(event EventBeginPlay)

(event Collision|EventActorBeginOverlap
  (params (OtherActor :type Actor%20Object%20Reference)))

(event EventTick
  (params (DeltaSeconds :type Float%20%28single-precision%29)))

(fn ConstructionScript)

(fn Setting
  (params (HP :type Float%20%28double-precision%29))
  (Variables|ATK|SetHit_Stack 0.0)
  (Variables|ATK|SetAtk_Delay_Time 0.0)
  (Variables|ATK|SetAtk_CoolTime false)
  (bind _outactors (Actor|GetAllActorsOfClass "/Game/ODH/BP/BP_PlayerRespawnPlace.BP_PlayerRespawnPlace_C"))
  (Variables|Respawn|SetRespawnPlace _outactors)
  (Variables|itAlive?|SetAlive true)
  (Variables|Respawn|SetRespawnDelayTime 0.0)
  (Variables|Respawn|SetRespawnCurrentTime 0.0)
  (Variables|Respawn|SetNowSpawn false)
  (Variables|Item|SetItemArray (Utilities|Array|MakeArray 0 0)))

(fn Respawn
  (params (Alive :type Boolean) (RespawnDelayTime :type Float%20%28double-precision%29) (Skeletal%20Mesh :type Skeletal%20Mesh%20Component%20Object%20Reference) (User :type Actor%20Object%20Reference))
  ;[0.15 0.15 0.15 0.5] 살아있는 상태인지 확인
  (if (not Alive)
    ;[0.15 0.15 0.15 0.5] 리스폰이 될때까지 시간이 걸리도록 만듦
    (bind _output_get (Variables|Respawn|SetRespawnDelayTime (+ RespawnDelayTime (Utilities|Time|GetWorldDeltaSeconds))))
    (if (>= _output_get 5.0)
      ;[0.15 0.15 0.15 0.5] 리스폰 지역 배열 중 랜덤으로 하나 선택, 해당 액터의 함수를 호출과 동시에 체력을 풀로 체움
      (bind _asbp_player_respawn_place (Utilities|Casting|CastToBP_PlayerRespawnPlace (.OutItem (Utilities|Array|Random (Variables|Respawn|GetRespawnPlace)))))
      (bind _asbp_player (Utilities|Casting|CastToBP_Player User)
        (:then
          (Default|SetHP _asbp_player)
          (Default|CharacterRespawn _asbp_player_respawn_place Alive _asbp_player_respawn_place)
          ;[0.15 0.15 0.15 0.5] 리스폰 무적시간 상태 체크
          (Variables|Respawn|SetNowSpawn true)
          ;[0.15 0.15 0.15 0.5] 리스폰 시 필요한 시간 리셋
          (Variables|Respawn|SetRespawnDelayTime 0.0)
          ;[0.15 0.15 0.15 0.5] 아이템 획득 상황 리셋
          (Variables|Item|SetItemArray (Utilities|Array|MakeArray 0 0))
          ;[0.15 0.15 0.15 0.5] 히트 스택 초기화
          (Variables|ATK|SetHit_Stack 0.0)
          (Rendering|SetVisibility Skeletal%20Mesh true false))
        (:CastFailed
          ;[0.15 0.15 0.15 0.5] 에너미에 체력 회복 이벤트를 추가해서 이를 불러오기
          (Utilities|Casting|CastToBP_DBS_Enemy_V User))))))

(fn CheckAlive
  (params (CheckAlive :type Boolean) (HP :type Float%20%28double-precision%29) (Who :type Actor%20Object%20Reference))
  ;[0.15 0.15 0.15 0.5] 살아있는 상태인지 확인
  (if CheckAlive
    ;[0.15 0.15 0.15 0.5] 체력이 0이 되면 생존 불을 false로 변경 아닐 경우 그대로 진행
    (if (<= HP 0.0)
      (bind _asbp_dbs_game (Utilities|Casting|CastToBP_DBS_Game (Game|GetGameMode)))
      (Default|PlayerDeadEvent _asbp_dbs_game 1)
      (bind _output_get (Variables|itAlive?|SetAlive false))
      (return _output_get)
      (else
        (bind _output_get_2 (Variables|itAlive?|SetAlive true))
        (return _output_get_2)))
    (else
      (bind _output_get_3 (Variables|itAlive?|SetAlive false))
      (return _output_get_3))))

(fn CheckNowSpawn
  (params (NowSpawn :type Boolean) (RespawnCurrentTime :type Float%20%28double-precision%29))
  ;[0.15 0.15 0.15 0.5] 리스폰 상태인지 체크하여 리스폰 상태일 경우 시간을 체크해서 일정 시간 이상이 되면 해제됨
  (if NowSpawn
    (bind _output_get (Variables|Respawn|SetRespawnCurrentTime (+ RespawnCurrentTime (Utilities|Time|GetWorldDeltaSeconds))))
    (if (>= _output_get 3.0)
      (Variables|Respawn|SetNowSpawn false)
      (Variables|Respawn|SetRespawnCurrentTime 0.0))))

(fn GetItem
  (params (Item :type Actor%20Object%20Reference) (ItmeUI :type WBP%20Item%20and%20Stack%20Object%20Reference))
  (bind _returnvalue (Utilities|GetClass Item))
  (bind _returnvalue_2 (Utilities|GetClass Item))
  (bind _itemarray (Variables|Item|GetItemArray))
  ;[0.15 0.15 0.15 0.5] 아이템 배열을 한바퀴 돌아서 빈 자리가 있으면 반복을 벗어난다
  (bind (_array_element _array_index) (Utilities|Array|ForEachLoopwithBreak _itemarray :!label _label)
    (:LoopBody
      (if (== _array_element 0)
        (goto _label Break)))
    (:Completed
      ;[0.15 0.15 0.15 0.5] 해당 위치에 아이템 셋팅
      (Utilities|Array|SetArrayElem _itemarray _array_index Item)
      ;[0.15 0.15 0.15 0.5] 인덱스 번호에 따라 설정되는 박스가 달라짐
      (if (== _array_index 0)
        ;[0.15 0.15 0.15 0.5] 0번 아이템 박스에 획득한 아이템에 따라 알맞은 이미지를 인벤토리에 설정
        (if (== _returnvalue_2 "/Game/ODH/BP/Item/Potion/BP_HPItem.BP_HPItem_C")
          (Variables|/Game/ODH/BP/WBP/WBP_ItemAndStack.WBP_ItemAndStack_C|SetBox_0_Items ItmeUI "NewEnumerator1")
          (elif (== _returnvalue_2 "/Game/ODH/BP/Item/Mine/BP_SpawnMineItem.BP_SpawnMineItem_C")
            (Variables|/Game/ODH/BP/WBP/WBP_ItemAndStack.WBP_ItemAndStack_C|SetBox_0_Items ItmeUI "NewEnumerator2")
            (else
              (Variables|/Game/ODH/BP/WBP/WBP_ItemAndStack.WBP_ItemAndStack_C|SetBox_0_Items ItmeUI "NewEnumerator0"))))
        (else
          ;[0.15 0.15 0.15 0.5] 1번 아이템 박스에 획득한 아이템에 따라 알맞은 이미지를 인벤토리에 설정
          (if (== _returnvalue "/Game/ODH/BP/Item/Potion/BP_HPItem.BP_HPItem_C")
            (Variables|/Game/ODH/BP/WBP/WBP_ItemAndStack.WBP_ItemAndStack_C|SetBox_1_Items ItmeUI "NewEnumerator1")
            (elif (== _returnvalue "/Game/ODH/BP/Item/Mine/BP_SpawnMineItem.BP_SpawnMineItem_C")
              (Variables|/Game/ODH/BP/WBP/WBP_ItemAndStack.WBP_ItemAndStack_C|SetBox_1_Items ItmeUI "NewEnumerator2")
              (else
                (Variables|/Game/ODH/BP/WBP/WBP_ItemAndStack.WBP_ItemAndStack_C|SetBox_1_Items ItmeUI "NewEnumerator0")))))))))

(fn UseHPItem
  (params (Item :type Actor%20Object%20Reference) (ItemUI :type WBP%20Item%20and%20Stack%20Object%20Reference))
  (bind _itemarray (Variables|Item|GetItemArray))
  (bind _returnvalue (Utilities|Array|FindItem _itemarray Item))
  ;[0.15 0.15 0.15 0.5] 아이템을 저장한 상태이며 그것이 체력 회복 아이템일 경우 체력을 회복시켜줌
  (if (!= Item 0)
    ;;[0.15 0.15 0.15 0.5] 아이템에 지정된 체력 회복 수치만큼 회복 시켜주고 아이템은 소멸, 만약 50보다 클 경우 50으로 됨
    (if (== (Utilities|GetClass Item) "/Game/ODH/BP/Item/Potion/BP_HPItem.BP_HPItem_C")
      ;;;[0.15 0.15 0.15 0.5] 자리가 0일 경우 첫번째 아이템 박스의 이미지 제거
      ;;; 아니면 두번째 아이템 박스 이미지 제거
      (if (== _returnvalue 0)
        (Variables|/Game/ODH/BP/WBP/WBP_ItemAndStack.WBP_ItemAndStack_C|SetBox_0_Items ItemUI "NewEnumerator0")
        (else
          (Variables|/Game/ODH/BP/WBP/WBP_ItemAndStack.WBP_ItemAndStack_C|SetBox_1_Items ItemUI "NewEnumerator0")))
      ;[0.15 0.15 0.15 0.5] 빈 배열을 생성 후 사용한 아이템 삭제
      (Utilities|Array|Insert _itemarray 0 _returnvalue)
      (Utilities|Array|RemoveIndex _itemarray _returnvalue)
      (return false)
      (else
        (return true)))))

(fn SetHitStack
  (params (NowHitStack :type Float%20%28double-precision%29))
  (Variables|ATK|SetHit_Stack (+ NowHitStack 1.0))
  (if (>= NowHitStack 6.0)
    (Variables|ATK|SetHit_Stack 6.0)))

(fn UseMineItem
  (params (Item :type Actor%20Object%20Reference) (NowLocal :type Vector) (UseActor :type Actor%20Object%20Reference) (ItemUI :type WBP%20Item%20and%20Stack%20Object%20Reference))
  (bind _returnvalue (Math|Conversions|ToTransform(Vector) NowLocal))
  (bind _itemarray (Variables|Item|GetItemArray))
  (bind _returnvalue_2 (Utilities|Array|FindItem _itemarray Item))
  (if (!= Item 0)
    ;[0.15 0.15 0.15 0.5] 해당 위치에 지뢰 아이템을 설치
    (if (== (Utilities|GetClass Item) "/Game/ODH/BP/Item/Mine/BP_SpawnMineItem.BP_SpawnMineItem_C")
      (bind _returnvalue_3 (Game|SpawnActorfromClass "/Game/ODH/BP/Item/Mine/BP_OnGroundMine.BP_OnGroundMine_C" (Math|Transform|MakeTransform (Math|Vector|MakeVector (.x (.location _returnvalue)) (.y (.location _returnvalue)) 0.0) "0, 0, 0" (.scale _returnvalue)) "Undefined" "MultiplyWithRoot" 0 0))
      ;;[0.15 0.15 0.15 0.5] 사용한 액터 전달
      (Default|UseMineItem _returnvalue_3 UseActor)
      ;[0.15 0.15 0.15 0.5] 자리가 0일 경우 첫번째 아이템 박스의 이미지 제거
      ; 아니면 두번째 아이템 박스 이미지 제거
      (if (== _returnvalue_2 0)
        (Variables|/Game/ODH/BP/WBP/WBP_ItemAndStack.WBP_ItemAndStack_C|SetBox_0_Items ItemUI "NewEnumerator0")
        (else
          (Variables|/Game/ODH/BP/WBP/WBP_ItemAndStack.WBP_ItemAndStack_C|SetBox_1_Items ItemUI "NewEnumerator0")))
      ;[0.15 0.15 0.15 0.5] 해당 아이템을 지우고 다시 빈자리를 만듦
      (Utilities|Array|Insert _itemarray 0 _returnvalue_2)
      (Utilities|Array|RemoveIndex _itemarray _returnvalue_2))))

(fn Healling
  (params (HP :type Float%20%28double-precision%29) (Healling :type Float%20%28double-precision%29) (BPCDamage :type BPC%20Damage%20System%20Object%20Reference))
  (bind _output_get (Variables|/Game/SSA/Interface/BPC_DamageSystem.BPC_DamageSystem_C|SetHealth BPCDamage (+ HP Healling)))
  (if (>= _output_get 5e+01)
    (Variables|/Game/SSA/Interface/BPC_DamageSystem.BPC_DamageSystem_C|SetHealth BPCDamage 5e+01)))