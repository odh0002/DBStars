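; BP_Test_DBS_Game is a test game-logic Blueprint that tracks player and enemy deaths and gates enemy respawning.
; On BeginPlay it creates the WBP_ScoreCopy widget and adds it to the viewport.
; PlayerDeadEvent and EnemyDeadEvent add to their death counters, while CastRespawnEnemy calls CallRespawnEnemy only when EnemeisAlive is zero.
; An EndGame timer and an enemy spawn-and-possess chain are left unconnected and never run.
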(event Custom|Cast%20Respawn%20Enemy
  (if (== (Variables|Default|GetEnemeisAlive) 0)
    (Default|CallRespawnEnemy)))

(event EventBeginPlay
  (bind _returnvalue (UserInterface|CreateWidget "/Game/ODH/BP/aTest/WBP_ScoreCopy.WBP_ScoreCopy_C"))
  (UserInterface|Viewport|AddtoViewport _returnvalue 0))

(event EventTick
  (params (DeltaSeconds :type Float%20%28single-precision%29)))

(fn ConstructionScript)

(fn PlayerDeadEvent
  (params (Count :type Integer))
  (Variables|Default|SetPlayerDead (+ Count (Variables|Default|GetPlayerDead))))

(fn EnemyDeadEvent
  (params (Count :type Integer))
  (Variables|Default|SetEnemyDead (+ Count (Variables|Default|GetEnemyDead))))