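; BP_GameManager is a game manager Blueprint that keeps a death score between the player and enemies and decides the match result.
; A DesthCount event increments the player's death count when the passed actor casts to BP_Player, otherwise the enemy's.
; GameEnd compares both counts, favors the side with fewer deaths, and prints Player Win, Enemy Win or Draw.
; Results and counts are only shown through debug PrintString.
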(event Custom|DesthCount
  (params (Who :type Actor%20Object%20Reference))
  ;[0.15 0.15 0.15 0.5] 누가 죽었는지 확인해서 만약 플레이어가 죽었을 경우 플레이어의 데스 카운트를 1 올림
  (Utilities|Casting|CastToBP_Player Who
    (:then
      (bind _output_get (Variables|Default|SetPlayerDeathCount (+ (Variables|Default|GetPlayerDeathCount) 1)))
      (Development|PrintString (Utilities|String|ToString(Integer) _output_get)))
    (:CastFailed
      ;[0.15 0.15 0.15 0.5] 에너미일 경우 에너미의 데스 카운트를 1올림
      (bind _output_get_2 (Variables|Default|SetEnemyDeathCount (+ (Variables|Default|GetEnemyDeathCount) 1)))
      (Development|PrintString (Utilities|String|ToString(Integer) _output_get_2) true true "(R=1.000000,G=0.000000,B=0.016369,A=1.000000)"))))

(event Custom|GameEnd
  ;[0.15 0.15 0.15 0.5] 시간이 종료됐을 때 에너미의 데스 카운트가 더 많으면 플레이어의 승리
  (if (> (Variables|Default|GetEnemyDeathCount) (Variables|Default|GetPlayerDeathCount))
    (Development|PrintString "Player Win")
    (else
      ;[0.15 0.15 0.15 0.5] 플레이어의 데스 카운트가 더 많으면 에너미의 승리
      (if (> (Variables|Default|GetPlayerDeathCount) (Variables|Default|GetEnemyDeathCount))
        (Development|PrintString "Enemy Win")
        (else
          ;[0.15 0.15 0.15 0.5] 동률일 경우 무승부
          (if (== (Variables|Default|GetPlayerDeathCount) (Variables|Default|GetEnemyDeathCount))
            (Development|PrintString "Draw")))))))

(event EventBeginPlay)

(event Collision|EventActorBeginOverlap
  (params (OtherActor :type Actor%20Object%20Reference)))

(event EventTick
  (params (DeltaSeconds :type Float%20%28single-precision%29)))

(fn ConstructionScript)