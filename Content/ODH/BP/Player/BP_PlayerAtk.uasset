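; BP_PlayerAtk is the player's attack projectile, flying forward at MoveSpeed until AliveTime expires.
; Each Tick it moves without sweep and runs a sphere trace, destroying itself on any hit or timeout.
; Hitting a BP_DBS_Enemy_V adds an attack stack on BP_Player, deals fixed damage through BPCDamageSystem, and notifies BP_Test_DBS_Game on a kill.
; The older overlap-based stack logic is disconnected.
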(event EventBeginPlay
  ;[0.15 0.15 0.15 0.5] 생성될때 플레이어의 클래스를 받음
  (bind _returnvalue (Actor|GetActorOfClass "/Game/ODH/BP/Player/BP_Player.BP_Player_C")))

(event Collision|EventActorBeginOverlap
  (params (OtherActor :type Actor%20Object%20Reference))
  ;[0.15 0.15 0.15 0.5] 아마 폐기?
  ;;[0.15 0.15 0.15 0.5] 에너미와 충돌시 스택을 쌓는 이벤트 호출 및 삭제
)

(event EventTick
  (params (DeltaSeconds :type Float%20%28single-precision%29))
  (bind _returnvalue (Transformation|GetActorLocation))
  ;[0.15 0.15 0.15 0.5] 공격 오브젝트가 앞으로 날아감
  (Variables|Default|SetCurrentTime (+ DeltaSeconds (Variables|Default|GetCurrentTime)))
  (Transformation|SetActorLocation (+ (Transformation|GetActorLocation) (* (* (Transformation|GetActorForwardVector) (Variables|Default|GetMove%20speed)) DeltaSeconds)) false false)
  ;[0.15 0.15 0.15 0.5] 투사체가 앞으로 계속 날아가면서
  ; 충돌을 하는지 파악을 함.
  (bind (_outhit _returnvalue_2) (Collision|SphereTraceForObjects _returnvalue _returnvalue 5e+01 (Utilities|Array|MakeArray "ObjectTypeQuery9") false 0 "None"))
  ;[0.15 0.15 0.15 0.5] 정해진 생존 시간보다 생존 시간이 적으면 계속 날아감
  (if (<= (Variables|Default|GetCurrentTime) (Variables|Default|GetAliveTime))
    ;[0.15 0.15 0.15 0.5] 충돌한 것이 에너미인지 파악
    (if _returnvalue_2
      (bind _asbp_dbs_enemy_v (Utilities|Casting|CastToBP_DBS_Enemy_V (.HitActor (Collision|BreakHitResult _outhit)))
        (:then
          (Default|AtkStackSet (stale EventBeginPlay _returnvalue))
          (Default|TakeDamage (Variables|/Game/SSA/Enemy/Villager/BP_DBS_Enemy_V.BP_DBS_Enemy_V_C|GetBPC_DamageSystem _asbp_dbs_enemy_v) (Utilities|Struct|MakeS_DamageInfo 6e+01 "NewEnumerator2" "NewEnumerator0" false))
          (if (<= (Variables|/Game/SSA/Interface/BPC_DamageSystem.BPC_DamageSystem_C|GetHealth (Variables|/Game/SSA/Enemy/Villager/BP_DBS_Enemy_V.BP_DBS_Enemy_V_C|GetBPC_DamageSystem _asbp_dbs_enemy_v)) 0.0)
            (bind _asbp_test_dbs_game (Utilities|Casting|CastToBP_Test_DBS_Game (Game|GetGameMode)))
            (Default|EnemyDeadEvent _asbp_test_dbs_game 1)
            (Actor|DestroyActor)
            (else
              (Actor|DestroyActor))))
        (:CastFailed
          ;[0.15 0.15 0.15 0.5] 생존 시간이 끝나거나 충돌한게 에너미가 아닐
          ; 경우 사라짐
          (Actor|DestroyActor :!label _label))))
    (else
      (goto _label))))

(fn ConstructionScript)