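; BP_SkillAtk is a thrown player skill projectile that tumbles in flight and bursts when it overlaps an actor.
; OnSkill takes the player and cursor positions, computes a high-arc toss velocity from Speed, then boosts the horizontal and reduces the vertical component to flatten the arc.
; On overlap, it spawns BP_SkillAtkEff for the area effect and damage, plays the Boom sound and destroys itself.
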(event Custom|OnSkill
  (params (PlayerPos :type Vector) (CursorPos :type Vector))
  (Variables|Default|SetStartPos PlayerPos)
  (Variables|Default|SetLastPos CursorPos)
  ;[0.15 0.15 0.15 0.5] 플레이어와 마우스 위치를 받아 해당 위치로 발사하게 만듦.
  (bind (_tossvelocity _returnvalue) (Class|GameplayStatics|BlueprintSuggestProjectileVelocity (Math|Vector|MakeVector (.x (Variables|Default|GetStartPos)) (.y (Variables|Default|GetStartPos)) 0.0) (Math|Vector|MakeVector (.x (Variables|Default|GetLastPos)) (.y (Variables|Default|GetLastPos)) 0.0) (Variables|Default|GetSpeed) 0.0 "DoNotTrace" 0.0 true false false))
  ;[0.15 0.15 0.15 0.5] z축이 너무 높아지기에 값을 조정해서 너무 높게 뜨지 않게 막음
  (if _returnvalue
    (Variables|/Script/Engine.MovementComponent|SetVelocity (Variables|Default|GetProjectileMovement) (Math|Vector|MakeVector (* (.x _tossvelocity) 1.6) (* (.y _tossvelocity) 1.6) (/ (.z _tossvelocity) 1.7)))))

(event EventBeginPlay)

(event Collision|EventActorBeginOverlap
  (params (OtherActor :type Actor%20Object%20Reference))
  (bind _returnvalue (Transformation|GetActorTransform))
  ;[0.15 0.15 0.15 0.5] 바닥에 부딪히면 범위에 이펙트와 대미지 판정 범위를 생성
  (Game|SpawnActorfromClass "/Game/ODH/BP/Player/BP_SkillAtkEff.BP_SkillAtkEff_C" (Math|Transform|MakeTransform (.location _returnvalue) "0, 0, 0" (.scale _returnvalue)) "Undefined" "MultiplyWithRoot" 0 0)
  (Audio|PlaySound2D "/Game/ODH/Sound/Boom.Boom" 1.0 1.0 0.0 0 0)
  (Actor|DestroyActor))

(event EventTick
  (params (DeltaSeconds :type Float%20%28single-precision%29))
  ;[0.15 0.15 0.15 0.5] 날아가는 동안 회전하게 만들기 위한 노드
  (Transformation|AddActorLocalRotation (Math|Rotator|MakeRotator (* 8e+01 DeltaSeconds) (* 8e+01 DeltaSeconds) (* 8e+01 DeltaSeconds)) false false))

(fn ConstructionScript)