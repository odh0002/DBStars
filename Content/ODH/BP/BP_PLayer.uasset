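; Top-down player pawn that turns to face the mouse cursor and spawns attacks.
; On BeginPlay it caches its BP_TopDownPlayerController, and each Tick it sets its yaw toward the cursor's Visibility hit point.
; Completing IA_PlayerAtk spawns BP_PlayerAtk at the AtkDirection component's transform.
; The CharaRotation function, which rotates only when not moving, and a debug line trace are left unconnected.
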(event Input|EnhancedActionEvents|EnhancedInputActionIA_PlayerAtk
  (params (ActionValue :type Boolean) (ElapsedSeconds :type Float%20%28double-precision%29) (TriggeredSeconds :type Float%20%28double-precision%29) (InputAction :type Input%20Action%20Object%20Reference :default "/Game/ODH/IA_PlayerAtk.IA_PlayerAtk"))
  (:Completed
    (Game|SpawnActorfromClass "/Game/ODH/BP/BP_PlayerAtk.BP_PlayerAtk_C" (Transformation|GetWorldTransform (Variables|Default|GetAtkDirection)) "AlwaysSpawn" "MultiplyWithRoot" 0 0)))

(event EventBeginPlay
  ;[0.15 0.15 0.15 0.5] Controller를 받아서 변수에 저장
  (bind _asbp_top_down_player_controller (Utilities|Casting|CastToBP_TopDownPlayerController (Pawn|GetController)))
  (Variables|Default|SetPlayer%20Cotroller _asbp_top_down_player_controller))

(event Collision|EventActorBeginOverlap
  (params (OtherActor :type Actor%20Object%20Reference)))

(event EventTick
  (params (DeltaSeconds :type Float%20%28single-precision%29))
  ;[0.15 0.15 0.15 0.5] 포인터와 캐릭터 간의 방향과 거리 시각화
  ;[0.15 0.15 0.15 0.5] 캐릭터가 마우스 포인터를 향해 바라봄
  (Transformation|SetActorRotation (Math|Rotator|MakeRotator 0.0 0.0 (.yaw (Math|Rotator|FindLookatRotation (Transformation|GetActorLocation) (.Location (Collision|BreakHitResult (.HitResult (Game|Player|GetHitResultUnderCursorbyChannel (Variables|Default|GetPlayer%20Cotroller) "TraceTypeQuery1" true)))))))))

(fn ConstructionScript)

(fn CharaRotation
  (params (NowMoving :type Boolean))
  (if (not NowMoving)
    ;[0.15 0.15 0.15 0.5] 캐릭터가 마우스 포인터를 향해 바라봄
    (Transformation|SetActorRotation (Math|Rotator|MakeRotator 0.0 0.0 (.yaw (Math|Rotator|FindLookatRotation (Transformation|GetActorLocation) (.Location (Collision|BreakHitResult (.HitResult (Game|Player|GetHitResultUnderCursorbyChannel (Variables|Default|GetPlayer%20Cotroller) "TraceTypeQuery1" true))))))))))