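; BP_PlayerAtk is a player attack projectile that flies forward and damages BP_StackTest actors it overlaps.
; Tick moves it along its forward vector at MoveSpeed without sweep and destroys it once its timer reaches AliveTime.
; On a hit, it calls AtkStackSet on the cached BP_Player and HpDown on the target, then destroys itself.
; HpDown receives a BP_PlayerAtk found by GetActorOfClass at BeginPlay, which may be another instance.
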(event EventBeginPlay
  ;[0.15 0.15 0.15 0.5] 생성될때 플레이어의 클래스를 받음
  (bind _returnvalue (Actor|GetActorOfClass "/Game/ODH/BP/BP_Player.BP_Player_C"))
  (bind _returnvalue_2 (Actor|GetActorOfClass "BP_PlayerAtk_C")))

(event Collision|EventActorBeginOverlap
  (params (OtherActor :type Actor%20Object%20Reference))
  ;[0.15 0.15 0.15 0.5] 에너미와 충돌시 스택을 쌓는 이벤트 호출 및 삭제
  (bind _asbp_stack_test (Utilities|Casting|CastToBP_StackTest OtherActor))
  ;;[0.15 0.15 0.15 0.5] 스택을 쌓는 이벤트 호출
  (Default|AtkStackSet (stale EventBeginPlay _returnvalue))
  (Default|HpDown _asbp_stack_test (stale EventBeginPlay _returnvalue_2))
  (Actor|DestroyActor))

(event EventTick
  (params (DeltaSeconds :type Float%20%28single-precision%29))
  ;[0.15 0.15 0.15 0.5] 공격 오브젝트가 앞으로 날아감
  (Variables|Default|SetCurrentTime (+ DeltaSeconds (Variables|Default|GetCurrentTime)))
  (Transformation|SetActorLocation (+ (Transformation|GetActorLocation) (* (* (Transformation|GetActorForwardVector) (Variables|Default|GetMove%20speed)) DeltaSeconds)) false false)
  (if (>= (Variables|Default|GetCurrentTime) (Variables|Default|GetAliveTime))
    (Actor|DestroyActor)))

(fn ConstructionScript)