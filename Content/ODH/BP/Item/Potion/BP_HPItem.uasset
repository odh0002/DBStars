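; BP_HPItem is an HP potion pickup that reacts when the player or an enemy overlaps it.
; BeginPlay caches the first BP_Player and BP_StackTest actors, and overlaps compare the first actor of the other actor's class against them.
; A player match passes a BP_HPItem found by class, plus the Healling value, to AddItem, then destroys the pickup.
; An enemy match only destroys it, without adding an item.
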(event EventBeginPlay
  ;[0.15 0.15 0.15 0.5] 플레이어 클래스를 미리 변수에 담아두기
  ; 나중 비교를 위한 작업
  (bind _returnvalue (Actor|GetActorOfClass "/Game/ODH/BP/Player/BP_Player.BP_Player_C"))
  (Variables|Default|SetPlayerActor _returnvalue)
  ;[0.15 0.15 0.15 0.5] 에너미 클래스를 미리 변수에 담아두기
  ; 나중 비교를 위한 작업
  (bind _returnvalue_2 (Actor|GetActorOfClass "/Game/ODH/BP/aTest/BP_StackTest.BP_StackTest_C"))
  (Variables|Default|SetEnemyActor _returnvalue_2))

(event Collision|EventActorBeginOverlap
  (params (OtherActor :type Actor%20Object%20Reference))
  ;[0.15 0.15 0.15 0.5] 부딪힌 액터의 클래스를 가져옴
  (bind _returnvalue (Actor|GetActorOfClass (Utilities|GetClass OtherActor)))
  ;[0.15 0.15 0.15 0.5] 플레이어 액터인지 비교
  (if (== _returnvalue (Variables|Default|GetPlayerActor))
    ;[0.15 0.15 0.15 0.5] 맞을 경우 플레이어에게 아이템을 추가해줌
    (bind _returnvalue_2 (Actor|GetActorOfClass "BP_HPItem_C"))
    (Default|AddItem (stale EventBeginPlay _returnvalue) _returnvalue_2 (Variables|Default|GetHealling))
    (Actor|DestroyActor)
    (else
      ;[0.15 0.15 0.15 0.5] 에너미에게 아이템을 추가하는 작업
      (if (== _returnvalue (Variables|Default|GetEnemyActor))
        (Actor|GetActorOfClass "BP_HPItem_C")
        (Actor|DestroyActor)))))

(event EventTick
  (params (DeltaSeconds :type Float%20%28single-precision%29)))

(fn ConstructionScript)