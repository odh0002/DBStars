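; BP_OnGroundMine is a placed mine item that explodes when a character other than its user overlaps it.
; BeginPlay enables collision and caches one BP_Player and one BP_DBS_Enemy_V, while UseMineItem records the user.
; On overlap with either cached actor, a sphere trace with persistent debug drawing gates fixed damage through that actor's BPCDamageSystem.
; The mine then spawns BP_MineBombEff and destroys itself.
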(event Custom|UseMineItem
  (params (UseCharactor :type Actor%20Object%20Reference))
  ;[0.15 0.15 0.15 0.5] 사용한 캐릭터의 클래스를 받는 이벤트
  (Variables|Default|SetUseCharacter UseCharactor))

(event EventBeginPlay
  ;[0.15 0.15 0.15 0.5] 바로 안터지게 생성때 콜리전을 킴
  (Collision|SetCollisionEnabled (Variables|Default|Getcollision) "QueryAndPhysics")
  (bind _returnvalue (Actor|GetActorOfClass "/Game/ODH/BP/Player/BP_Player.BP_Player_C"))
  (bind _output_get (Variables|Default|SetPlayer _returnvalue))
  (bind _returnvalue_2 (Actor|GetActorOfClass "/Game/SSA/Enemy/Villager/BP_DBS_Enemy_V.BP_DBS_Enemy_V_C"))
  (Variables|Default|SetEnemy _returnvalue_2))

(event Collision|EventActorBeginOverlap
  (params (OtherActor :type Actor%20Object%20Reference))
  (bind _returnvalue (Transformation|GetActorLocation))
  (bind _returnvalue_2 (Transformation|GetActorLocation))
  ;[0.15 0.15 0.15 0.5] 설치한 캐릭터가 아닌 캐릭터와 충돌이 일어났을 경우 자신 위치에 폭발과 대미지가 일어난다
  (if (!= OtherActor (Variables|Default|GetUseCharacter))
    (if (== OtherActor (Variables|Default|GetPlayer))
      (bind (_outhit _returnvalue_3) (Collision|SphereTraceForObjects _returnvalue _returnvalue 125.0 (Utilities|Array|MakeArray "ObjectTypeQuery7") false 0 "Persistent"))
      (if _returnvalue_3
        (Default|TakeDamage (Variables|/Game/ODH/BP/Player/BP_Player.BP_Player_C|GetBPC_DamageSystem (Variables|Default|GetPlayer)) (Utilities|Struct|MakeS_DamageInfo 15.0 "NewEnumerator2" "NewEnumerator0" false))
        (Game|SpawnActorfromClass "/Game/ODH/BP/Item/Mine/BP_MineBombEff.BP_MineBombEff_C" (Transformation|GetActorTransform) "Undefined" "MultiplyWithRoot" 0 0)
        (Actor|DestroyActor))
      (else
        ;[0.15 0.15 0.15 0.5] 에너미 대미지 이벤트 호출
        (if (== OtherActor (Variables|Default|GetEnemy))
          (bind (_outhit_2 _returnvalue_4) (Collision|SphereTraceForObjects _returnvalue_2 _returnvalue_2 125.0 (Utilities|Array|MakeArray "ObjectTypeQuery9") false 0 "Persistent"))
          (if _returnvalue_4
            (Default|TakeDamage (Variables|/Game/SSA/Enemy/Villager/BP_DBS_Enemy_V.BP_DBS_Enemy_V_C|GetBPC_DamageSystem (Variables|Default|GetEnemy)) (Utilities|Struct|MakeS_DamageInfo 15.0 "NewEnumerator2" "NewEnumerator0" false))
            (Game|SpawnActorfromClass "/Game/ODH/BP/Item/Mine/BP_MineBombEff.BP_MineBombEff_C" (Transformation|GetActorTransform) "Undefined" "MultiplyWithRoot" 0 0)
            (Actor|DestroyActor)))))))

(event EventTick
  (params (DeltaSeconds :type Float%20%28single-precision%29)))

(fn ConstructionScript)