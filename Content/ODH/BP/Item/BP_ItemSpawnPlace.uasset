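; BP_ItemSpawnPlace is an item spawn point that creates a random pickup when BP_ItemSpawnManager signals it.
; On BeginPlay it caches the level's BP_HPItem and BP_OtherItem instances found by GetActorOfClass as templates for their classes.
; SignalItemSpawnPlace forwards a boolean and target actor to ItemSpawn.
; When true, ItemSpawn spawns a randomly chosen instance's class at a random point in a small box around that target.
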(event Custom|Signal%20Item%20Spawn%20Place
  (params (SetTime :type Boolean) (SpawnPlace :type Actor%20Object%20Reference))
  ;[0.15 0.15 0.15 0.5] BP_ItemSpawnManager 에서 아이템 생성하라는
  ; 신호를 받아서 아이템 생성 함수 실행
  (CallFunction|ItemSpawn SetTime SpawnPlace))

(event EventBeginPlay
  ;[0.15 0.15 0.15 0.5] 아이템 클래스들을 미리 배열에 저장해둠
  ; 후에 저장해둔 배열에서 아이템을 랜덤하게 뽑기 위한 작업
  (bind _returnvalue (Actor|GetActorOfClass "/Game/ODH/BP/Item/BP_HPItem.BP_HPItem_C"))
  (bind _returnvalue_2 (Actor|GetActorOfClass "/Game/ODH/BP/Item/BP_OtherItem.BP_OtherItem_C"))
  (Variables|Default|SetItemClass (Utilities|Array|MakeArray _returnvalue _returnvalue_2)))

(event Collision|EventActorBeginOverlap
  (params (OtherActor :type Actor%20Object%20Reference)))

(event EventTick
  (params (DeltaSeconds :type Float%20%28single-precision%29)))

(fn ConstructionScript)

(fn ItemSpawn
  (params (SpanwTrue :type Boolean) (SpawnPlace :type Actor%20Object%20Reference))
  (if SpanwTrue
    ;[0.15 0.15 0.15 0.5] 해당 위치에 랜덤하게 뽑힌 아이템을 생성
    (Game|SpawnActorfromClass (Utilities|GetClass (.OutItem (Utilities|Array|Random (Variables|Default|GetItemClass)))) (Math|Conversions|ToTransform(Vector) (Math|Random|RandomPointinBoundingBox (Transformation|GetActorLocation SpawnPlace) (Math|Vector|MakeVector 2e+01 2e+01 0.0))) "Undefined" "MultiplyWithRoot" 0 0)))