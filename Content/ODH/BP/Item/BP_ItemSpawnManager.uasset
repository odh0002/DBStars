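; BP_ItemSpawnManager is a manager actor that periodically triggers item spawns at random spawn points in the level.
; On BeginPlay it caches every BP_ItemSpawnPlace actor in an array.
; Tick accumulates time until it reaches Delay, then signals one random spawn place via SignalItemSpawnPlace, resets the timer and rolls a new random delay, printing it to screen.
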(event EventBeginPlay
  ;[0.15 0.15 0.15 0.5] 아이템이 스폰 가능하도록 한 actor의 클래스를 전부 배열에 저장
  (bind _outactors (Actor|GetAllActorsOfClass "/Game/ODH/BP/Item/BP_ItemSpawnPlace.BP_ItemSpawnPlace_C"))
  (Variables|Default|SetItemSpawnPlace _outactors))

(event Collision|EventActorBeginOverlap
  (params (OtherActor :type Actor%20Object%20Reference)))

(event EventTick
  (params (DeltaSeconds :type Float%20%28single-precision%29))
  ;[0.15 0.15 0.15 0.5] 스폰 시간이 지나면 아이템을 생성하게 체크함
  (bind _output_get (Variables|Default|SetCurrentTime (+ (Variables|Default|GetCurrentTime) (Utilities|Time|GetWorldDeltaSeconds))))
  (if (>= _output_get (Variables|Default|GetDelay))
    ;[0.15 0.15 0.15 0.5] 미리 저장한 아이템 스폰 배열에서 랜덤으로 하나를 추출.
    ; 해당 actor에게 아이템 스폰 이벤트를 실행하게 함.
    (bind _asbp_item_spawn_place (Utilities|Casting|CastToBP_ItemSpawnPlace (.OutItem (Utilities|Array|Random (Variables|Default|GetItemSpawnPlace)))))
    (Default|SignalItemSpawnPlace _asbp_item_spawn_place (>= _output_get (Variables|Default|GetDelay)) _asbp_item_spawn_place)
    ;[0.15 0.15 0.15 0.5] 아이템 스폰 시간 랜덤 지정
    ;;[0.15 0.15 0.15 0.5] 현재 시간 리셋
    (Variables|Default|SetCurrentTime 0.0)
    (bind _output_get_2 (Variables|Default|SetDelay (Math|Random|RandomFloatinRange 2e+01 45.0)))
    (Development|PrintString (Utilities|String|ToString(Float) _output_get_2) true true "(R=0.000000,G=0.660000,B=1.000000,A=1.000000)" 4.0)))

(fn ConstructionScript)